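; Interactable lower-left cabinet door Blueprint that swings open and closed on its static mesh.
; BeginPlay caches the mesh's relative rotation, and each Interaction alternately plays or reverses the OpenClose timeline, lerping yaw to 90 degrees past that start.
; OnLooking enables custom depth rendering as a highlight while Tick clears it every frame, so it shows only while looking events keep firing.
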(event EventBeginPlay
  (|CallParentFunction)
  (Variables|Default|SetRotation (Variables|/Script/Engine.SceneComponent|GetRelativeRotation (Variables|Default|GetStaticMesh))))

(event Collision|EventActorBeginOverlap
  (params (OtherActor :type Actor%20Object%20Reference))
  (|CallParentFunction OtherActor) ; This node is disabled and will not be called.\nDrag off pins to build functionality.
)

(event EventInteraction
  (params (Player :type BP%20First%20Person%20Character%20Object%20Reference) (Inventory :type AC%20Inventory%20Object%20Reference))
  (bind _rotation (Variables|Default|GetRotation))
  (bind (_roll _pitch _yaw) (Math|Rotator|BreakRotator _rotation))
  (Utilities|FlowControl|FlipFlop
    (:A
      (bind _newtrack_0 (Timeline|OpenClose Play)
        (:Update
          (Transformation|SetRelativeRotation (Variables|Default|GetStaticMesh) (Math|Rotator|Lerp(Rotator) _rotation (Math|Rotator|MakeRotator _roll _pitch (+ _yaw 9e+01)) _newtrack_0) false false))))
    (:B
      (Timeline|OpenClose Reverse))))

(event EventOnLooking
  (Rendering|SetRenderCustomDepth (Variables|Default|GetStaticMesh) true))

(event EventTick
  (params (DeltaSeconds :type Float%20%28single-precision%29))
  (Rendering|SetRenderCustomDepth (Variables|Default|GetStaticMesh) false))

(fn ConstructionScript
  (|CallParentFunction))