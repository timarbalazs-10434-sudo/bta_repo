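; BP_WardrobeWall02B is a post-Soviet wardrobe wall furniture prop with adjustable doors and drawers.
; The Construction Script yaws the left and right door meshes by LeftDoor and RightDoor, and slides three drawer meshes along local Y by DrawerTop, DrawerMid and DrawerBottom.
; Posing happens only at construction, as relative local rotations and offsets; the event graph holds no logic.
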(event EventBeginPlay)

(event Collision|EventActorBeginOverlap
  (params (OtherActor :type Actor%20Object%20Reference)))

(event EventTick
  (params (DeltaSeconds :type Float%20%28single-precision%29)))

(fn ConstructionScript
  (Utilities|FlowControl|Sequence
    (:then_0
      (Transformation|AddLocalRotation (Variables|Default|GetSM_WardrobeWallll_02_Door_03) (Math|Rotator|MakeRotator 0.0 0.0 (Variables|Default|GetLeft_Door)) false false))
    (:then_1
      (Transformation|AddLocalRotation (Variables|Default|GetStaticMesh2) (Math|Rotator|MakeRotator 0.0 0.0 (Variables|Default|GetRight_Door)) false false))
    (:then_2
      (Transformation|AddLocalOffset (Variables|Default|GetStaticMeshComponent02) (Math|Vector|MakeVector 0.0 (Variables|Default|GetDrawer_Top) 0.0) false false))
    (:then_3
      (Transformation|AddLocalOffset (Variables|Default|GetStaticMesh) (Math|Vector|MakeVector 0.0 (Variables|Default|GetDrawer_Mid) 0.0) false false))
    (:then_4
      (Transformation|AddLocalOffset (Variables|Default|GetStaticMesh1) (Math|Vector|MakeVector 0.0 (Variables|Default|GetDrawer_Bottom) 0.0) false false))))