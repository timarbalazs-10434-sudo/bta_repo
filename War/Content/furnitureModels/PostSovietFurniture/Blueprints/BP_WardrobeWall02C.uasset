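; Post-Soviet wardrobe wall furniture prop with five individually posable mesh parts, likely doors.
; The Construction Script adds a local rotation to each part from its own angle variable: yaw for the top and bottom left and right parts, roll for the middle one.
; The event graph holds only disabled stub events, so the pose is set at construction with no runtime interaction.
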(event EventBeginPlay)

(event Collision|EventActorBeginOverlap
  (params (OtherActor :type Actor%20Object%20Reference)))

(event EventTick
  (params (DeltaSeconds :type Float%20%28single-precision%29)))

(fn ConstructionScript
  (Utilities|FlowControl|Sequence
    (:then_0
      (Transformation|AddLocalRotation (Variables|Default|GetStaticMeshComponent0) (Math|Rotator|MakeRotator 0.0 0.0 (Variables|Default|GetTop_Left)) false false))
    (:then_1
      (Transformation|AddLocalRotation (Variables|Default|GetStaticMesh) (Math|Rotator|MakeRotator 0.0 0.0 (Variables|Default|GetTop_Right)) false false))
    (:then_2
      (Transformation|AddLocalRotation (Variables|Default|GetStaticMeshComponent01) (Math|Rotator|MakeRotator (Variables|Default|GetMiddle) 0.0 0.0) false false))
    (:then_3
      (Transformation|AddLocalRotation (Variables|Default|GetStaticMeshComponent03) (Math|Rotator|MakeRotator 0.0 0.0 (Variables|Default|GetBotton_Left)) false false))
    (:then_4
      (Transformation|AddLocalRotation (Variables|Default|GetStaticMesh1) (Math|Rotator|MakeRotator 0.0 0.0 (Variables|Default|GetBotton_Right)) false false))))