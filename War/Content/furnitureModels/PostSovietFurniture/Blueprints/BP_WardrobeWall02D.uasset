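; BP_WardrobeWall02D is a post-Soviet wardrobe wall furniture prop with adjustable door angles.
; Its construction script adds yaw rotation to three door mesh components from the Door, BottomLeft and BottomRight variables, so each can be posed separately in the editor.
; The event graph holds only disabled default events, so it has no runtime behaviour.
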(event EventBeginPlay)

(event Collision|EventActorBeginOverlap
  (params (OtherActor :type Actor%20Object%20Reference)))

(event EventTick
  (params (DeltaSeconds :type Float%20%28single-precision%29)))

(fn ConstructionScript
  (Utilities|FlowControl|Sequence
    (:then_0
      (Transformation|AddLocalRotation (Variables|Default|GetStaticMeshComponent04) (Math|Rotator|MakeRotator 0.0 0.0 (Variables|Default|GetDoor)) false false))
    (:then_1
      (Transformation|AddLocalRotation (Variables|Default|GetSM_WardrobeWallll_02_Door_04) (Math|Rotator|MakeRotator 0.0 0.0 (Variables|Default|GetBottom_Left)) false false))
    (:then_2
      (Transformation|AddLocalRotation (Variables|Default|GetStaticMesh) (Math|Rotator|MakeRotator 0.0 0.0 (Variables|Default|GetBottom_Right)) false false))))