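; BP_RussianSoldier is a modular Russian soldier character assembled from separate skeletal mesh parts.
; The construction script makes the boots, fur, gloves, night vision, head and balaklava follow the main Mesh's pose through master pose.
; An eye-blink timeline is wired to drive the Mesh's eyes_blink morph target and replay after random pauses, but nothing starts it, so it never runs.
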(fn ConstructionScript
  (Class|SkinnedMeshComponent|SetMasterPoseComponent (Variables|Default|Getboots) (Variables|Character|GetMesh) false))