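; BP_WardrobeWall01B is a wardrobe wall furniture prop with four adjustable doors: upper left, upper right, lower left and lower right.
; The Construction Script adds a local yaw rotation to each door component from its own float variable, so each door's opening angle is set independently at construction time.
; The Event Graph holds only disabled placeholder events, so the Blueprint has no runtime interaction or animation.
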(event EventBeginPlay)

(event Collision|EventActorBeginOverlap
  (params (OtherActor :type Actor%20Object%20Reference)))

(event EventTick
  (params (DeltaSeconds :type Float%20%28single-precision%29)))

(fn ConstructionScript
  (Utilities|FlowControl|Sequence
    (:then_0
      (Transformation|AddLocalRotation (Variables|Default|GetWardrobeWall01_ADD1) (Math|Rotator|MakeRotator 0.0 0.0 (Variables|Default|GetUp_Left_Door)) false false))
    (:then_1
      (Transformation|AddLocalRotation (Variables|Default|GetWardrobeWall01_ADD) (Math|Rotator|MakeRotator 0.0 0.0 (Variables|Default|GetUp_Right_Door)) false false))
    (:then_2
      (Transformation|AddLocalRotation (Variables|Default|GetWardrobeWall01_b_ADD) (Math|Rotator|MakeRotator 0.0 0.0 (Variables|Default|GetDown_Left_Door)) false false))
    (:then_3
      (Transformation|AddLocalRotation (Variables|Default|GetWardrobeWall01_b_ADD1) (Math|Rotator|MakeRotator 0.0 0.0 (Variables|Default|GetDown_Right_Door)) false false))))