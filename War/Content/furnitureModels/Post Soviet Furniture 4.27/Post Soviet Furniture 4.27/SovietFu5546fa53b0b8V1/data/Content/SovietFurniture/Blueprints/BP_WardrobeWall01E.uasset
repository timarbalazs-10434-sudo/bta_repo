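; BP_WardrobeWall01E is a Soviet furniture wardrobe wall prop with adjustable door positions.
; The Construction Script rotates one mesh component in yaw by UpDoor and slides three others along local Y by the DownDoor variables.
; Posing happens only at construction, as the event graph holds only disabled placeholder events with no runtime logic.
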(event EventBeginPlay)

(event Collision|EventActorBeginOverlap
  (params (OtherActor :type Actor%20Object%20Reference)))

(event EventTick
  (params (DeltaSeconds :type Float%20%28single-precision%29)))

(fn ConstructionScript
  (Utilities|FlowControl|Sequence
    (:then_0
      (Transformation|AddLocalRotation (Variables|Default|GetStaticMeshComponent04) (Math|Rotator|MakeRotator 0.0 0.0 (Variables|Default|GetUpDoor)) false false))
    (:then_1
      (Transformation|AddLocalOffset (Variables|Default|GetStaticMeshComponent01) (Math|Vector|MakeVector 0.0 (Variables|Default|GetDown_Door01) 0.0) false false))
    (:then_2
      (Transformation|AddLocalOffset (Variables|Default|GetStaticMeshComponent02) (Math|Vector|MakeVector 0.0 (Variables|Default|GetDown_Door02) 0.0) false false))
    (:then_3
      (Transformation|AddLocalOffset (Variables|Default|GetStaticMeshComponent03) (Math|Vector|MakeVector 0.0 (Variables|Default|GetDown_Door03) 0.0) false false))))