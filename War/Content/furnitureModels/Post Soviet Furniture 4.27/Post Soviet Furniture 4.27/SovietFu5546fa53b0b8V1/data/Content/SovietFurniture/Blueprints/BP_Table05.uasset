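; BP_Table05 is a table prop Blueprint, from a Soviet furniture pack, with three drawers that can be posed open or closed.
; Its construction script offsets three static mesh components along local Y using the DrawerTop, DrawerMid and DrawerDown variables.
; The event graph holds only disabled default events, so the drawers have no runtime behavior.
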(event EventBeginPlay)

(event Collision|EventActorBeginOverlap
  (params (OtherActor :type Actor%20Object%20Reference)))

(event EventTick
  (params (DeltaSeconds :type Float%20%28single-precision%29)))

(fn ConstructionScript
  (Utilities|FlowControl|Sequence
    (:then_0
      (Transformation|AddLocalOffset (Variables|Default|GetStaticMeshComponent0) (Math|Vector|MakeVector 0.0 (Variables|Default|GetDrawer_Top) 0.0) false false))
    (:then_1
      (Transformation|AddLocalOffset (Variables|Default|GetStaticMeshComponent01) (Math|Vector|MakeVector 0.0 (Variables|Default|GetDrawer_Mid) 0.0) false false))
    (:then_2
      (Transformation|AddLocalOffset (Variables|Default|GetStaticMesh) (Math|Vector|MakeVector 0.0 (Variables|Default|GetDrawer_Down) 0.0) false false))))