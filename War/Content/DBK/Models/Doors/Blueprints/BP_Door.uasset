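; BP_Door is an interactable door that swings open and closed with attenuated, randomly pitched sounds.
; Each Interaction alternates a FlipFlop between playing and reversing a Timeline, which lerps the root between two fixed world rotations, regardless of placed orientation.
; OnLooking enables custom depth on the mesh and Tick clears it every frame, so the highlight lasts only while that event keeps firing.
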(event EventTick
  (params (DeltaSeconds :type Float%20%28single-precision%29))
  (Rendering|SetRenderCustomDepth (Variables|Default|GetStaticMesh) false))

(event EventBeginPlay)

(event Collision|EventActorBeginOverlap
  (params (OtherActor :type Actor%20Object%20Reference)))

(event EventInteraction
  (params (Player :type BP%20First%20Person%20Character%20Object%20Reference) (Inventory :type AC%20Inventory%20Object%20Reference))
  (Utilities|FlowControl|FlipFlop
    (:A
      (Audio|PlaySoundatLocation "/Game/Sounds/doorOpenSound.doorOpenSound" (Transformation|GetWorldLocation (Variables|Default|GetDefaultSceneRoot)) "0, 0, 0" 1.0 (Math|Random|RandomFloatinRange 1.3 0.95) 0.0 "/Game/FirstPerson/Blueprints/SoundSystem/SoundAttenuation.SoundAttenuation" 0 0 0)
      (bind _newtrack_0 (Timeline|Timeline Play)
        (:Update
          (Transformation|SetWorldRotation (Variables|Default|GetDefaultSceneRoot) (Math|Rotator|Lerp(Rotator) "0.000000,270.000000,0.000000" "0.000000,180.000000,0.000000" _newtrack_0) false false))))
    (:B
      (Audio|PlaySoundatLocation "/Game/Sounds/doorCloseSound.doorCloseSound" (Transformation|GetWorldLocation (Variables|Default|GetDefaultSceneRoot)) "0, 0, 0" 1.0 (Math|Random|RandomFloatinRange 1.3 0.95) 0.0 "/Game/FirstPerson/Blueprints/SoundSystem/SoundAttenuation.SoundAttenuation" 0 0 0)
      (Timeline|Timeline Reverse))))

(event EventOnLooking
  (Rendering|SetRenderCustomDepth (Variables|Default|GetStaticMesh) true))

(fn ConstructionScript)